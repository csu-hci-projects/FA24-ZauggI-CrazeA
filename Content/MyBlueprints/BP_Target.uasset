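; BP_Target is a shootable target that the player eliminates with first-person projectiles.
; Each projectile hit subtracts a fixed amount from HitPoints.
; When HitPoints reaches exactly zero, it spawns an explosion at the hit location, increments the player character's TargetsEliminated count, calls its CheckLevelComplete, and destroys itself.
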(event Collision|EventHit
  (params (MyComp :type Primitive%20Component%20Object%20Reference) (Other :type Actor%20Object%20Reference) (OtherComp :type Primitive%20Component%20Object%20Reference) (bSelfMoved :type Boolean) (HitLocation :type Vector :default "0, 0, 0") (HitNormal :type Vector :default "0, 0, 0") (NormalImpulse :type Vector :default "0, 0, 0") (Hit :type Hit%20Result%20Structure%20%28by%20ref%29))
  (Utilities|Casting|CastToBP_FirstPersonProjectile Other)
  (bind _output_get (Variables|Default|SetHitPoints (- (Variables|Default|GetHitPoints) 20)))
  (if (== _output_get 0)
    (Effects|SpawnEmitteratLocation "/Game/StarterContent/Particles/P_Explosion.P_Explosion" HitLocation)
    (bind _asbp_first_person_character (Utilities|Casting|CastToBP_FirstPersonCharacter (Game|GetPlayerCharacter 0)))
    (Math|Integer|IncrementInt (Variables|/Game/FirstPerson/Blueprints/BP_FirstPersonCharacter.BP_FirstPersonCharacter_C|GetTargetsEliminated _asbp_first_person_character)
      (:%20%20
        (Default|CheckLevelComplete _asbp_first_person_character)
        (Actor|DestroyActor)))))

(fn ConstructionScript)