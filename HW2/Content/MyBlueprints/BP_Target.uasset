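; BP_Target is a shootable target actor that takes two Projectile hits to destroy.
; On overlap with a Projectile it counts the hit, swapping its mesh to the TargetHit material on the first.
; On the next hit it spawns an explosion, has the player's VRPawn show a popup via OnTargetDestroyed, calls CallTargetDestroyed and destroys itself.
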(event Custom|OnTargetDestroyed
  ;[1 1 1] Destroy Target (Second Hit)
  (bind _asvrpawn (Utilities|Casting|CastToVRPawn (Game|Player|GetPlayerPawn 0)))
  (Default|ShowPopup _asvrpawn))

(event Collision|EventActorBeginOverlap
  (params (OtherActor :type Actor%20Object%20Reference))
  (Utilities|Casting|CastToProjectile OtherActor)
  (bind _result (Math|Integer|IncrementInt (Variables|Default|GetHits))
    (:%20%20
      (if (== _result 1)
        ;[1 1 1] Change Material (First Hit)
        (Rendering|Material|SetMaterial (Variables|Default|GetStaticMesh) 0 "/Game/StarterContent/Materials/TargetHit.TargetHit")
        (else
          ;[1 1 1] Destroy Target (Second Hit)
          (Effects|SpawnEmitteratLocation "/Game/StarterContent/Particles/P_Explosion.P_Explosion" (Transformation|GetWorldLocation (Variables|Default|GetStaticMesh)))
          (CallFunction|OnTargetDestroyed)
          (Default|CallTargetDestroyed)
          (Actor|DestroyActor))))))

(fn ConstructionScript)